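; BP_BasePawn is a pawn that rolls like a cube, tipping 90 degrees over a bottom edge per move.
; Move input snaps to its dominant axis and is ignored while a roll timer runs.
; Each roll stores the mesh center and pivots around an offset from it by cube dimensions and direction.
; A looping ~60 Hz timer rotates location and orientation in MaxSteps increments, drawing the pivot as a debug sphere.
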(event `EnhancedInput|/Game/Blueprints/Input/Actions/IA_Move`
  (params (ActionValue :type "Vector2D Structure") (ElapsedSeconds :type "Float (double-precision)") (TriggeredSeconds :type "Float (double-precision)") (InputAction :type "InputAction Object Reference" :default "/Game/Blueprints/Input/Actions/IA_Move.IA_Move"))
  (bind (_x _y) (`KismetMathLibrary.BreakVector2D` ActionValue))
  (bind _returnvalue (* _y -1.0))
  (:`Triggered`
    (`self.CheckMovement` (select `bool` (>= (`KismetMathLibrary.Abs` _x) (`KismetMathLibrary.Abs` _returnvalue)) :`false` (`KismetMathLibrary.MakeVector2D` 0.0 _returnvalue) :`true` (`KismetMathLibrary.MakeVector2D` _x) :!type "Vector2D Structure"))))

(event `CheckMovement`
  (params (InputValue :type "Vector2D Structure"))
  (if (not (`KismetSystemLibrary.K2_IsTimerActive` null "MoveArroundPivot"))
    (set `self.Input Value` InputValue)
    (set `self.LastPosition` (`KismetSystemLibrary.GetComponentBounds` (`self.StaticMesh`)))
    (`KismetSystemLibrary.K2_SetTimer` null "MoveArroundPivot" 0.0166 true)))

(fn `GetPivotPoint`
  (returns (PivotPoint :type "Vector Structure"))
  (locals (LocalPivot :type "Vector Structure"))
  (bind (_cubedimension_x _cubedimension_y _cubedimension_z) (`KismetMathLibrary.BreakVector` (`self.CubeDimension`)))
  (bind _localpivot (`local.LocalPivot`))
  (bind (_x _y) (`KismetMathLibrary.BreakVector2D` (`self.Input Value`)))
  (set `local.LocalPivot` (+ (`self.LastPosition`) (`KismetMathLibrary.MakeVector` (* _cubedimension_x _x) (* _cubedimension_y _y) (* _cubedimension_z -1.0))))
  (`KismetSystemLibrary.DrawDebugSphere` _localpivot 15.0 12 (struct :`R` 1.0 :`A` 1.0) 1.0 3.0)
  (return _localpivot))

(fn `MoveArroundPivot`
  (locals (StepPercent :type "Float (double-precision)"))
  (bind (_x _y) (`KismetMathLibrary.BreakVector2D` (`self.Input Value`)))
  (bind _returnvalue (`KismetMathLibrary.MakeVector` (* _y -1.0) _x))
  (bind _returnvalue_2 (* (/ 1.0 (`KismetMathLibrary.Conv_IntToDouble` (`self.MaxSteps`))) 90.0))
  (if (< (`self.CurrentStep`) (`self.MaxSteps`))
    (`self.K2_SetActorLocationAndRotation` (+ (`KismetMathLibrary.RotateAngleAxis` (- (`self.K2_GetActorLocation`) (`self.GetPivotPoint`)) _returnvalue_2 _returnvalue) (`self.GetPivotPoint`)) (`KismetMathLibrary.ComposeRotators` (`self.K2_GetActorRotation`) (`KismetMathLibrary.RotatorFromAxisAndAngle` _returnvalue _returnvalue_2)))
    (`/Engine/EditorBlueprintResources/StandardMacros.IncrementInt` (`self.CurrentStep`)
      (:`  `
        _))
    (else
      (`KismetSystemLibrary.K2_ClearTimer` null "MoveArroundPivot")
      (set `self.CurrentStep` 0)))
  (return))

(fn `UserConstructionScript`)